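; NPC Blueprint for a simple dialogue system that opens a choices menu when the player presses E nearby.
; Box overlap enables input and opens a Gate for the E key; leaving closes it and removes all widgets.
; Each accepted press alternates through a FlipFlop between showing the Choices01 widget with a mouse cursor and restoring unpaused, game-only input with the cursor hidden.
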(event `Key|E`
  (params (Key :type "Key Structure" :default "AnyKey"))
  (bind _returnvalue (`GameplayStatics.GetPlayerController` 0))
  (:`Pressed`
    (`/Engine/EditorBlueprintResources/StandardMacros.Gate` true :!label _label
      (:`Exit`
        (`/Engine/EditorBlueprintResources/StandardMacros.FlipFlop`
          (:`A`
            (set `PlayerController.bShowMouseCursor` true (`GameplayStatics.GetPlayerController` 0))
            (bind _returnvalue_2 (`|CreateWidget` "/Game/SimpleDialogSystem/Widgets/Basic_Dialog/Choices/Choices01.Choices01_C"))
            (`UserWidget.AddToViewport` _returnvalue_2 0))
          (:`B`
            (`GameplayStatics.SetGamePaused` false)
            (`self.EnableInput` _returnvalue null)
            (set `PlayerController.bShowMouseCursor` false _returnvalue)
            (`WidgetBlueprintLibrary.SetInputMode_GameOnly` _returnvalue)))))))

(event `self.Box.OnComponentBeginOverlap`
  (params (OtherActor :type "Actor Object Reference") (OtherComp :type "PrimitiveComponent Object Reference") (OtherBodyIndex :type Integer) (bFromSweep :type Boolean) (SweepResult :type "HitResult Structure (by ref)"))
  (`self.EnableInput` (`GameplayStatics.GetPlayerController` 0))
  (goto _label :!via `Open`))

(event `self.Box.OnComponentEndOverlap`
  (params (OtherActor :type "Actor Object Reference") (OtherComp :type "PrimitiveComponent Object Reference") (OtherBodyIndex :type Integer))
  (`WidgetLayoutLibrary.RemoveAllWidgets`)
  (goto _label :!via `Close`))

(fn `UserConstructionScript`)